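; BP_Player is the first-person player for the BlockBreaker level, handling movement, mouse-style look, shooting and pausing.
; On BeginPlay it spawns a BP_Rifle and snaps it to the GunLocation component.
; The Shoot axis fires the gun along the camera's forward vector, with a CanShoot flag and Delay enforcing the gun's fire rate.
; Escape drives a FlipFlop that toggles the PauseMenu widget, game pause and cursor visibility.
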(event `InputAxis|Move_Forward`
  (params (AxisValue :type "Float (single-precision)"))
  ;[1 1 1] Move Forward/Backwards
  (`self.AddMovementInput` (`self.GetActorForwardVector`) AxisValue))

(event `InputAxis|Move_Right`
  (params (AxisValue :type "Float (single-precision)"))
  ;[1 1 1] Move Right/Left
  (`self.AddMovementInput` (`self.GetActorRightVector`) AxisValue))

(event `InputAxis|LookHorizontal`
  (params (AxisValue :type "Float (single-precision)"))
  ;[1 1 1] LookHorizontal
  (`self.AddControllerYawInput` AxisValue))

(event `InputAxis|LookVertical`
  (params (AxisValue :type "Float (single-precision)"))
  ;[1 1 1] LookVertical
  (`self.AddControllerPitchInput` (* AxisValue -1.0)))

(event `self.ReceiveBeginPlay`
  ;[1 1 1] Spawning and attaching gun
  (bind _returnvalue (`|SpawnActorFromClass` "/Game/Levels/BlockBreaker/Blueprints/BP_Rifle.BP_Rifle_C" (`KismetMathLibrary.MakeTransform` (0.0 0.0 0.0)) "Undefined" "OverrideRootScale" null null))
  (bind _output_get (set `self.EquippedGun` _returnvalue))
  (`self.K2_AttachToComponent` _output_get (`self.GunLocation`) "None" "SnapToTarget" "SnapToTarget" "KeepRelative" true))

(event `InputAxis|Shoot`
  (params (AxisValue :type "Float (single-precision)"))
  (bind _fpscamera (`self.FpsCamera`))
  (bind _returnvalue (`SceneComponent.K2_GetComponentLocation` _fpscamera))
  ;[1 1 1] Shooting + Firerate
  (if (and (== AxisValue 1.0) (`self.Can Shoot`))
    (`/Game/Levels/BlockBreaker/Blueprints/BP_BaseGun.Shoot` (`self.EquippedGun`) _returnvalue (+ _returnvalue (* (`SceneComponent.GetForwardVector` _fpscamera) (`/Game/Levels/BlockBreaker/Blueprints/BP_BaseGun.MaximumBulletDistance` (`self.EquippedGun`)))))
    (set `self.Can Shoot` false)
    (`KismetSystemLibrary.Delay` (`/Game/Levels/BlockBreaker/Blueprints/BP_BaseGun.FireRate` (`self.EquippedGun`)))
    (set `self.Can Shoot` true)))

(event `Key|Escape` :paused true
  (params (Key :type "Key Structure"))
  (bind _returnvalue (`GameplayStatics.GetPlayerController` 0))
  ;[1 1 1] Pause Game
  (:`Pressed`
    (`/Engine/EditorBlueprintResources/StandardMacros.FlipFlop`
      (:`A`
        (bind _returnvalue_2 (`|CreateWidget` "/Game/MostUI/PauseMenu.PauseMenu_C"))
        (`UserWidget.AddToViewport` _returnvalue_2 0)
        (`GameplayStatics.SetGamePaused` true)
        (set `PlayerController.bShowMouseCursor` true _returnvalue))
      (:`B`
        (`Widget.RemoveFromParent` _returnvalue_2)
        (`GameplayStatics.SetGamePaused` false)
        (set `PlayerController.bShowMouseCursor` false _returnvalue)))))

(fn `UserConstructionScript`)